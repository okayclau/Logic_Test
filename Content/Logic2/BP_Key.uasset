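; BP_Key is a key actor that comes in Tutorial, Lvl1 and Lvl2 variants.
; Its construction script picks the KeyMesh from the KeyType value, then runs the parent construction script.
; BeginPlay only calls the parent, and the overlap and tick events are disabled, so this Blueprint adds no runtime logic of its own.
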(event `self.ReceiveBeginPlay`
  (`parent.ReceiveBeginPlay`))

(fn `UserConstructionScript`
  (set `self.Key Mesh` (select `/Game/Logic2/E_KeyType` (`self.Key Type`) :`NewEnumerator0` (`self.Tutorial`) :`NewEnumerator1` (`self.Lvl 1`) :`NewEnumerator2` (`self.Lvl 2`)))
  (`parent.UserConstructionScript`))