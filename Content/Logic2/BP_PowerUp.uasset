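; BP_PowerUp is a power-up pickable that comes in speed, size and invincibility variants (Velocidad, Grande, Invencibilidad).
; Its construction script sets PowerUpMesh from PowerUpType and assigns a fixed PickableType before calling the parent construction script.
; BeginPlay only calls the parent, and overlap and Tick are disabled stubs, so this Blueprint adds no pickup or effect logic of its own.
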(event `self.ReceiveBeginPlay`
  (`parent.ReceiveBeginPlay`))

(fn `UserConstructionScript`
  (set `self.Power Up Mesh` (select `/Game/Logic2/E_PowerUpType` (`self.PowerUp Type`) :`NewEnumerator0` (`self.Velocidad`) :`NewEnumerator1` (`self.Grande`) :`NewEnumerator2` (`self.Invencibilidad`)))
  (set `self.PickableType` "NewEnumerator2")
  (`parent.UserConstructionScript`))