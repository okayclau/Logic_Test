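; BP_DAKS_Player is a player Blueprint that collects pickable items on contact.
; When CollisionComponent begins an overlap, it casts the other actor to BP_Pickable and branches on its PickableType.
; Key, Coin and Power Up each cast to their own subclass, print the specific type and destroy the item.
; Pickups are only printed on screen, with no inventory, score or effect applied here.
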(event `self.CollisionComponent.OnComponentBeginOverlap`
  (params (OverlappedComponent :type "PrimitiveComponent Object Reference") (OtherActor :type "Actor Object Reference") (OtherComp :type "PrimitiveComponent Object Reference") (OtherBodyIndex :type Integer) (bFromSweep :type Boolean) (SweepResult :type "HitResult Structure (by ref)"))
  (bind _asbp_pickable (cast `/Game/Logic2/BP_Pickable` OtherActor))
  (switch `/Game/Logic2/E_PickableType` (`/Game/Logic2/BP_Pickable.PickableType` _asbp_pickable)
    (:`NewEnumerator0`
      ; ñ
      (bind _asbp_key (cast `/Game/Logic2/BP_Key` OtherActor))
      (`KismetSystemLibrary.PrintString` (`KismetStringLibrary.Concat_StrStr` "Key Picked" (`|GetEnumeratorNameAsString` (`/Game/Logic2/BP_Key.Key Type` _asbp_key))))
      (`self.K2_DestroyActor` OtherActor))
    (:`NewEnumerator1`
      (bind _asbp_coin (cast `/Game/Logic2/BP_Coin` OtherActor))
      (`KismetSystemLibrary.PrintString` (`KismetStringLibrary.Concat_StrStr` "Coin Picked" (`|GetEnumeratorNameAsString` (`/Game/Logic2/BP_Coin.CoinType` _asbp_coin))))
      (`self.K2_DestroyActor` OtherActor))
    (:`NewEnumerator2`
      (bind _asbp_power_up (cast `/Game/Logic2/BP_PowerUp` OtherActor))
      (`KismetSystemLibrary.PrintString` (`KismetStringLibrary.Concat_StrStr` "PowerUp Picked -> " (`|GetEnumeratorNameAsString` (`/Game/Logic2/BP_PowerUp.PowerUp Type` _asbp_power_up))))
      (`self.K2_DestroyActor` OtherActor))))

(fn `UserConstructionScript`)