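; BP_Moneda is a coin pickup with an animated mesh and an overlap trigger.
; Tick calls Play on a Timeline whose Progreso track lerps SMMoneda's relative transform from TransformDeMoneda to MovVertical.
; Any overlap on MonedaCol increments the Blueprint's own ContadorMonedas, then destroys the collider and mesh components, leaving the actor itself in place.
; BeginPlay sets MonedaActiva, which this graph never reads.
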(event `self.ReceiveBeginPlay`
  (set `self.monedaActiva` true))

(event `self.ReceiveTick`
  (params (DeltaSeconds :type "Float (single-precision)"))
  (bind (_direction _progreso) (`Timeline|Timeline` :`NewTime` 5.0)
    (:`Update`
      (`SceneComponent.K2_SetRelativeTransform` (`self.SM_Moneda`) (`KismetMathLibrary.TLerp` (`self.TransformDeMoneda`) (`self.MovVertical`) _progreso) false false))))

(event `self.MonedaCol.OnComponentBeginOverlap`
  (params (OverlappedComponent :type "PrimitiveComponent Object Reference") (OtherActor :type "Actor Object Reference") (OtherComp :type "PrimitiveComponent Object Reference") (OtherBodyIndex :type Integer) (bFromSweep :type Boolean) (SweepResult :type "HitResult Structure (by ref)"))
  (set `self.ContadorMonedas` (+ (`self.ContadorMonedas`) 1))
  (`ActorComponent.K2_DestroyComponent` (`self.MonedaCol`))
  (`ActorComponent.K2_DestroyComponent` (`self.SM_Moneda`)))

(fn `UserConstructionScript`)