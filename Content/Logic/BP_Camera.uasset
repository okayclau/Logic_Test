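; BP_Camera is a camera actor that takes over the first player controller's view and follows the third-person character along Y and Z.
; On BeginPlay it finds BP_ThirdPersonCharacter and caches its CamTarget component.
; Each Tick it eases toward that target with FInterpTo, faster vertically than horizontally, keeping its own X fixed.
; An older capsule-offset follow with rotation adjustment remains disconnected.
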(event `self.ReceiveBeginPlay`
  (`PlayerController.SetViewTargetWithBlend` (`GameplayStatics.GetPlayerController` 0) self 0.0 "VTBlend_Linear" 0.0 false)
  (bind _returnvalue (`GameplayStatics.GetActorOfClass` "/Game/ThirdPerson/Blueprints/BP_ThirdPersonCharacter.BP_ThirdPersonCharacter_C"))
  (set `self.Cam Target` (`/Game/ThirdPerson/Blueprints/BP_ThirdPersonCharacter.CamTarget` _returnvalue)))

(event `self.ReceiveTick`
  (params (DeltaSeconds :type "Float (single-precision)"))
  (bind (_returnvalue_x _returnvalue_y _returnvalue_z) (`KismetMathLibrary.BreakVector` (`self.K2_GetActorLocation`)))
  (bind _returnvalue (`GameplayStatics.GetWorldDeltaSeconds`))
  (bind (_returnvalue_x_2 _returnvalue_y_2 _returnvalue_z_2) (`KismetMathLibrary.BreakVector` (`SceneComponent.K2_GetComponentLocation` (`self.Cam Target`))))
  (bind _returnvalue_2 (`KismetMathLibrary.FInterpTo` _returnvalue_y _returnvalue_y_2 _returnvalue 2.0))
  ; forma de deewa
  (`self.K2_SetActorLocation` (`KismetMathLibrary.MakeVector` _returnvalue_x _returnvalue_2 (`KismetMathLibrary.FInterpTo` _returnvalue_z _returnvalue_z_2 _returnvalue 5.0)))
  (set `self.Current` _returnvalue_2))

(fn `UserConstructionScript`)