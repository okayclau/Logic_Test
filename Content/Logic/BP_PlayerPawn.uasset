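; BP_PlayerPawn is a player pawn Blueprint that currently holds only setup and debug overlap logic.
; On BeginPlay it finds BP_UIManager in the level and caches its HUD reference.
; Its CollisionComponent overlap casts the other actor to DefaultPawn and prints whether the cast and reference are valid.
; Tick is empty, and a disconnected fragment would call OverlapMoney on a Door_And_Key actor but never runs.
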(event `self.ReceiveBeginPlay`
  (bind _returnvalue (`GameplayStatics.GetActorOfClass` "/Game/Logic/BP_UIManager.BP_UIManager_C"))
  (set `self.HUD` (`/Game/Logic/BP_UIManager.HUD` _returnvalue)))

(event `self.ReceiveTick`
  (params (DeltaSeconds :type "Float (single-precision)")))

(event `self.CollisionComponent.OnComponentBeginOverlap`
  (params (OverlappedComponent :type "PrimitiveComponent Object Reference") (OtherActor :type "Actor Object Reference") (OtherComp :type "PrimitiveComponent Object Reference") (OtherBodyIndex :type Integer) (bFromSweep :type Boolean) (SweepResult :type "HitResult Structure (by ref)"))
  ; comprueba si el tipo de actor e4s defauktpawn
  (bind _asdefault_pawn (cast `DefaultPawn` OtherActor)
    (:`then`
      (`/Engine/EditorBlueprintResources/StandardMacros.IsValid` _asdefault_pawn
        (:`Is Valid`
          (`KismetSystemLibrary.PrintString` "todo OK"))
        (:`Is Not Valid`
          (`KismetSystemLibrary.PrintString` "ref de pawn lost"))))
    (:`CastFailed`
      (`KismetSystemLibrary.PrintString` "mal"))))

(fn `UserConstructionScript`)